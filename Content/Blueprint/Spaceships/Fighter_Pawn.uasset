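; Player-controlled spaceship fighter pawn with six-degree-of-freedom physics flight and a first/third-person view toggle.
; Movement and rotation axis inputs add linear or angular velocity to BodyMesh along its local axes, except Up/Down, which uses the actor's up vector.
; Forward movement and roll use the mesh's right vector, while strafe and pitch use its forward vector.
; ChangeView flip-flops which view component is active.
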(event Input|ActionEvents|InputActionChangeView
  (params (Key :type Key%20Structure))
  (:Pressed
    (Utilities|FlowControl|FlipFlop
      (:A
        (Components|Activation|SetActive (Variables|Default|GetFirstperson) true false)
        (Components|Activation|SetActive (Variables|Default|GetThirdperson) false true))
      (:B
        (Components|Activation|SetActive (Variables|Default|GetThirdperson) true false)
        (Components|Activation|SetActive (Variables|Default|GetFirstperson) false true)))))

(event Input|AxisEvents|InputAxisUp/Down
  (params (AxisValue :type Float%20%28single-precision%29))
  ;[1 1 1] Ship Mouvement
  (Physics|SetPhysicsLinearVelocity (Variables|Default|GetBodyMesh) (* (Math|Vector|GetUpVector (Transformation|GetActorRotation)) (* AxisValue 5.0)) true "None"))

(event Input|AxisEvents|InputAxisLookUpAxis
  (params (AxisValue :type Float%20%28single-precision%29))
  (bind _bodymesh (Variables|Default|GetBodyMesh))
  ;[1 1 1] Ship Mouvement
  (Class|PrimitiveComponent|SetPhysicsAngularVelocityinDegrees _bodymesh (* (Math|Vector|GetForwardVector (Transformation|GetWorldRotation _bodymesh)) (* AxisValue 0.05)) true "None"))

(event Input|AxisEvents|InputAxisTurn
  (params (AxisValue :type Float%20%28single-precision%29))
  (bind _bodymesh (Variables|Default|GetBodyMesh))
  ;[1 1 1] Ship Mouvement
  (Class|PrimitiveComponent|SetPhysicsAngularVelocityinDegrees _bodymesh (* (Math|Vector|GetUpVector (Transformation|GetWorldRotation _bodymesh)) (* AxisValue 0.05)) true "None"))

(event Input|AxisEvents|InputAxisMoveForwardAxis
  (params (AxisValue :type Float%20%28single-precision%29))
  (bind _bodymesh (Variables|Default|GetBodyMesh))
  ;[1 1 1] Ship Mouvement
  (Physics|SetPhysicsLinearVelocity _bodymesh (* (Math|Vector|GetRightVector (Transformation|GetWorldRotation _bodymesh)) (* AxisValue 1e+01)) true "None"))

(event Input|AxisEvents|InputAxisRoll
  (params (AxisValue :type Float%20%28single-precision%29))
  (bind _bodymesh (Variables|Default|GetBodyMesh))
  ;[1 1 1] Ship Mouvement
  (Class|PrimitiveComponent|SetPhysicsAngularVelocityinDegrees _bodymesh (* (Math|Vector|GetRightVector (Transformation|GetWorldRotation _bodymesh)) (* AxisValue -0.5)) true "None"))

(event Input|AxisEvents|InputAxisMoveRightAxis
  (params (AxisValue :type Float%20%28single-precision%29))
  (bind _bodymesh (Variables|Default|GetBodyMesh))
  ;[1 1 1] Ship Mouvement
  (Physics|SetPhysicsLinearVelocity _bodymesh (* (Math|Vector|GetForwardVector (Transformation|GetWorldRotation _bodymesh)) (* AxisValue 1e+01)) true "None"))

(fn ConstructionScript)