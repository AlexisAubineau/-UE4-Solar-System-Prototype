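; Earths is a planet actor that orbits horizontally around a target actor, or around its own starting location if no valid target is set.
; Each Tick advances the rotation by speed and delta time, signed by the Clockwise flag.
; RotateActorAroundPoint rotates a radius vector around the Z axis from a starting angle, adds it to the center and moves the actor there.
; An optional debug line links center and planet.
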(event EventBeginPlay
  (Variables|Default|SetInitialLocation (Transformation|GetActorLocation)))

(event EventTick
  (params (DeltaSeconds :type Float%20%28single-precision%29))
  (Variables|Default|SetCurrentRotation (+ (Variables|Default|GetCurrentRotation) (* (* (Variables|Default|GetRotationSpeed) DeltaSeconds) (Math|Float|SelectFloat 1.0 -1.0 (Variables|Default|GetClockwise)))))
  (bind _newparam (CallFunction|RotateActorAroundPoint self (Variables|Default|GetTargetActor) (Variables|Default|GetInitialLocation) (Variables|Default|GetRadius) (Variables|Default|GetStartingAngle) (Variables|Default|GetCurrentRotation)))
  (if (Variables|Default|GetDrawDebug)
    (Rendering|Debug|DrawDebugLine _newparam (Transformation|GetActorLocation) (Variables|Default|GetTraceColor) 1.0 2.0)))

(fn ConstructionScript)

(fn RotateActorAroundPoint
  (params (ActorToRotate :type Actor%20Object%20Reference) (TargetActor :type Actor%20Object%20Reference) (LocationTarget :type Vector) (Radius :type Float%20%28single-precision%29) (Angles :type Float%20%28single-precision%29) (RotationRate :type Float%20%28single-precision%29))
  (LocalVariables|SetLActorToRotate ActorToRotate)
  (LocalVariables|SetLTargetActor TargetActor)
  (LocalVariables|SetLLocation LocationTarget)
  (LocalVariables|SetLoRadius Radius)
  (LocalVariables|SetLAngle Angles)
  (LocalVariables|SetLRate RotationRate)
  (Utilities|IsValid (LocalVariables|GetLTargetActor)
    (:Is%20Valid
      (LocalVariables|SetLLocation (Transformation|GetActorLocation (LocalVariables|GetLTargetActor))))
    (:Is%20Not%20Valid
      _))
  (Transformation|SetActorLocation (LocalVariables|GetLActorToRotate) (+ (LocalVariables|GetLLocation) (Math|Vector|RotateVectorAroundAxis (Math|Vector|MakeVector (LocalVariables|GetLoRadius) 0.0 0.0) (+ (LocalVariables|GetLRate) (LocalVariables|GetLAngle)) "0, 0,1.000000")) false false)
  (return (LocalVariables|GetLLocation)))